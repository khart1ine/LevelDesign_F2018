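; BP_MovingPlatform1 is a platform that shuttles its static mesh between a start and end position, optionally looping.
; After an initial delay on BeginPlay, a custom event chains timed MoveComponentTo calls with pauses at each end, calling itself again while looping is enabled.
; The construction script uses self-resetting booleans as editor buttons, capturing the actor's current location as either endpoint.
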(event Custom|GoToLocationAndBack
  (bind _returnvalue (Transformation|GetActorRotation))
  ;[1 1 1] Move Platform Back and Forth
  (Components|MoveComponentTo (Variables|Debug|GetStaticMeshComponent) (Variables|Platform|GetEnd%20Position) _returnvalue false false (Variables|Platform|GetSpeed) false)
  (Utilities|FlowControl|Delay (Variables|Platform|GetDelay))
  (Components|MoveComponentTo (Variables|Debug|GetStaticMeshComponent) (Variables|Platform|GetStart%20Position) _returnvalue false false (Variables|Platform|GetSpeed) false)
  (Utilities|FlowControl|Delay (Variables|Platform|GetDelay))
  (if (Variables|Platform|GetPlatform%20Is%20Looping?)
    (CallFunction|GotoLocationandBack)))

(event EventBeginPlay
  ;[1 1 1] Move Platform
  (Utilities|FlowControl|Delay (Variables|Platform|GetDelay))
  (CallFunction|GotoLocationandBack))

(event Collision|EventActorBeginOverlap
  (params (OtherActor :type Actor%20Object%20Reference)))

(event EventTick
  (params (DeltaSeconds :type Float%20%28single-precision%29)))

(fn ConstructionScript
  (bind _returnvalue (Transformation|GetActorLocation))
  ;[1 1 1] Set Start and End Location of Platform
  (Utilities|FlowControl|Sequence
    (:then_0
      (if (Variables|Platform|GetSet%20Start%20Position)
        (Variables|Platform|SetStart%20Position _returnvalue)
        (Variables|Platform|SetSet%20Start%20Position false)))
    (:then_1
      (if (Variables|Platform|GetSet%20End%20Position)
        (Variables|Platform|SetEnd%20Position _returnvalue)
        (Variables|Platform|SetSet%20End%20Position false)))))